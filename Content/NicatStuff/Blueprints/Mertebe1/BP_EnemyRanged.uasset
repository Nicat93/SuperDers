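; BP_EnemyRanged is a ranged enemy that chases the player and shoots with a weapon component attached to its GripPoint socket.
; A latent AIMoveTo loop brings it within range, stores the aim direction, turns it toward the player, fires, plays a montage, then repeats after a delay.
; GetAimDirection exposes that vector, while ammo and weapon queries return fixed values.
; When health depletes, it drops its capsule, ragdolls and is destroyed after a delay.
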(event OnDamageDepleted(BPC_Health)
  (bind _mesh (Variables|Character|GetMesh))
  (bind _capsulecomponent (Variables|Collision|GetCapsuleComponent)
    (:then
      (Components|DestroyComponent _capsulecomponent))
    (:else
      _))
  (Physics|SetSimulatePhysics _mesh true)
  (Collision|SetCollisionEnabled _mesh "QueryAndPhysics")
  (Utilities|FlowControl|Delay 5.0)
  (Actor|DestroyActor))

(event EventBeginPlay
  (bind _returnvalue (Transformation|GetActorLocation))
  (bind _returnvalue_2 (Game|GetPlayerCharacter 0))
  (bind _returnvalue_3 (Transformation|GetActorLocation _returnvalue_2))
  (bind _returnvalue_4 (AddComponent|AddBPWeaponComponent false))
  (Variables|Default|SetWeapon _returnvalue_4)
  (Transformation|AttachComponentToComponent _returnvalue_4 (Variables|Character|GetMesh) "GripPoint" "SnapToTarget" "SnapToTarget" "SnapToTarget" true)
  (AI|AIMoveTo self "0, 0, 0" (Game|GetPlayerCharacter 0) (Variables|Default|GetAcceptance%20Radius) false :!label _label
    (:OnSuccess
      (Utilities|IsValid (Game|GetPlayerCharacter 0)
        (:Is%20Valid
          (Variables|Default|SetAimDirectionVector (Math|Vector|GetUnitDirection(Vector) _returnvalue _returnvalue_3))
          (Transformation|SetActorRotation (Math|Rotator|CombineRotators "0.000000,-45.000000,0.000000" (Math|Rotator|FindLookatRotation _returnvalue _returnvalue_3)))
          (Default|EventFireWeapon (Variables|Default|GetWeapon))
          (Animation|Montage|PlayMontage (Variables|Character|GetMesh) "/Game/FirstPersonArms/Animations/FP_Rifle_Shoot_Montage.FP_Rifle_Shoot_Montage"
            (:OnCompleted
              _)))))
    (:OnFail
      _))
  (Utilities|FlowControl|Delay (Variables|Default|GetFireLoopDelay))
  (Utilities|IsValid (Game|GetPlayerCharacter 0)
    (:Is%20Valid
      (goto _label))))

(fn ConstructionScript)

(fn GetAimDirection
  (return (Variables|Default|GetAimDirectionVector) false))

(fn GetAmmoCount
  (return 0))

(fn HasWeapon
  (return true))