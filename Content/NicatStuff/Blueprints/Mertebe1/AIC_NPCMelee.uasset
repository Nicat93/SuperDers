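; AI controller for a melee NPC that starts the BT_NPCMelee behavior tree on BeginPlay.
; Its AI Perception update events are bound but empty, so the controller leaves the NPC's behavior to the tree.
; Disconnected leftover graphs would print perceived actors, or poll a large sphere overlap for BP_FirstPersonCharacter to set the TargetEnemy blackboard key, but neither runs.
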(event OnPerceptionUpdated(AIPerception)
  (params (UpdatedActors :type Array%20of%20Actor%20Object%20References)))

(event OnTargetPerceptionUpdated(AIPerception)
  (params (Actor :type Actor%20Object%20Reference) (Stimulus :type AI%20Stimulus%20Structure)))

(event OnTargetPerceptionInfoUpdated(AIPerception)
  (params (UpdateInfo :type Actor%20Perception%20Update%20Info%20Structure%20%28by%20ref%29)))

(event EventBeginPlay
  (AI|RunBehaviorTree "/Game/NicatStuff/BehaviorTree/BT_NPCMelee.BT_NPCMelee"))

(fn ConstructionScript)