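; BP_EnemyMelee is a melee zombie enemy that kicks the player and dies when its health component depletes.
; Its attack event plays a kick montage, applies damage to the first player character on the HitNotify notify without a range check, and sends an AI message when the montage completes.
; On depletion it destroys its capsule, ragdolls the mesh with physics and collision, and destroys itself five seconds later.
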(event OnDamageDepleted(BPC_Health)
  (bind _mesh (Variables|Character|GetMesh))
  (bind _capsulecomponent (Variables|Collision|GetCapsuleComponent)
    (:then
      (Components|DestroyComponent _capsulecomponent))
    (:else
      _))
  (Physics|SetSimulatePhysics _mesh true)
  (Collision|SetCollisionEnabled _mesh "QueryAndPhysics")
  (Utilities|FlowControl|Delay 5.0)
  (Actor|DestroyActor))

(event Custom|EventZombieAttack
  (bind _notifyname (Animation|Montage|PlayMontage (Variables|Character|GetMesh) "/Game/NicatStuff/TEST/ZombieKicking_UE_Montage.ZombieKicking_UE_Montage")
    (:OnCompleted
      (Class|AIBlueprintHelperLibrary|SendAIMessage self (GameplayTags|GetTagName (GameplayTags|MakeLiteralGameplayTag "(TagName=\"AI.Messages.AttackFinished\")")) 0 true))
    (:OnNotifyBegin
      (if (== _notifyname "HitNotify")
        (Game|Damage|ApplyDamage (Game|GetPlayerCharacter 0) 1.0 0 0)))))

(fn ConstructionScript)