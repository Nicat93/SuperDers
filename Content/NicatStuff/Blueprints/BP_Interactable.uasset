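; BP_Interactable is a base interactable that gates and routes interaction requests into empty Interact and EndInteraction events, which serve as hooks for specific behavior.
; TryInteract checks the interactor's tag against a whitelist with exact matching.
; In toggle mode each accepted attempt flips IsInteracting, seeded from a starting state, to start or end interaction.
; Otherwise TryInteract always fires Interact, and TryEndInteraction fires EndInteraction without tracking state.
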(event Custom|TryEndInteraction
  (if (not (Variables|Default|GetbToggledInteraction))
    (CallFunction|EndInteraction)))

(event Custom|TryInteract
  (params (Interactor :type Gameplay%20Tag%20Structure))
  (if (GameplayTags|MatchesAnyTags Interactor (Variables|Default|GetInteractorWhitelist) true)
    (if (Variables|Default|GetbToggledInteraction)
      (if (Variables|Default|GetbIsInteracting)
        (Variables|Default|SetbIsInteracting false)
        (CallFunction|EndInteraction)
        (else
          (Variables|Default|SetbIsInteracting true)
          (CallFunction|Interact Interactor)))
      (else
        (CallFunction|Interact Interactor)))))

(event Custom|Interact
  (params (Interactor :type Gameplay%20Tag%20Structure)))

(event Custom|EndInteraction)

(event EventBeginPlay
  (Variables|Default|SetbIsInteracting (Variables|Default|GetbStartingInteractionState)))

(fn ConstructionScript)