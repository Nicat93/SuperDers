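; BP_Light is an interactable light that switches its point light on during an interaction and off when the interaction ends.
; The Interact and EndInteraction events call TurnOn and TurnOff, which set the TurnedOn flag and apply it to the PointLight's visibility.
; The construction script only calls its parent.
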(event Custom|TurnOn
  (Variables|Default|SetbTurnedOn true)
  (Rendering|SetVisibility (Variables|Default|GetPointLight) (Variables|Default|GetbTurnedOn) false))

(event Custom|TurnOff
  (Variables|Default|SetbTurnedOn false)
  (Rendering|SetVisibility (Variables|Default|GetPointLight) (Variables|Default|GetbTurnedOn) false))

(event EventInteract
  (params (Interactor :type Gameplay%20Tag%20Structure))
  (CallFunction|Turnon))

(event EventEndInteraction
  (CallFunction|TurnOff))

(fn ConstructionScript
  (|CallParentFunction))