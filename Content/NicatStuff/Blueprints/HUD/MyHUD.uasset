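; MyHUD is a HUD Blueprint that draws a center-screen square, likely a crosshair, with a text label below it.
; BeginPlay also adds a UMG_Test widget to the viewport.
; Each DrawHUD resets RectColor to red and clears Text after drawing, so any other values must be set again every frame.
; Nodes for UI-only input and a visible cursor are present but never run.
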(event EventBeginPlay
  (bind _returnvalue (UserInterface|CreateWidget "/Game/NicatStuff/TEST/UMG_Test.UMG_Test_C"))
  (UserInterface|Viewport|AddtoViewport _returnvalue 0))

(event EventDrawHUD
  (params (SizeX :type Integer) (SizeY :type Integer))
  (bind _returnvalue (/ SizeY 2))
  (bind _returnvalue_2 (/ SizeX 2))
  (bind _returnvalue_3 (Math|Conversions|ToFloat(Integer) _returnvalue_2))
  (bind _returnvalue_4 (Math|Conversions|ToFloat(Integer) _returnvalue))
  (HUD|DrawRect (Variables|Default|GetRectColor) _returnvalue_3 _returnvalue_4 1e+01 1e+01)
  (Variables|Default|SetRectColor "(R=1.000000,G=0.000000,B=0.000000,A=1.000000)")
  (HUD|DrawText (Variables|Default|GetText) "(R=1.000000,G=1.000000,B=1.000000,A=1.000000)" (+ _returnvalue_3 -3e+01) (+ _returnvalue_4 25.0) 0 2.0 false)
  (Variables|Default|SetText ""))

(fn ConstructionScript)