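; BPC_Interactor is an actor component that lets its owner interact with objects held in an Interactables collection.
; Interact tries to interact through Interactables, passing the Interactor, but only when the collection is not empty.
; EndInteraction forwards a request to end the interaction.
; A GetInteractorTag function exists but shows no returned value.
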(event EventInteract
  (params (Interactor :type Gameplay%20Tag%20Structure))
  (if (Utilities|Array|IsNotEmpty (Variables|Default|GetInteractables))
    (Default|TryInteract (Variables|Default|GetInteractables) (Variables|Default|GetInteractor))))

(event EventEndInteraction
  (Default|TryEndInteraction (Variables|Default|GetInteractables)))

(fn GetInteractorTag
  (return ""))