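; BP_OverlapTrigger is a trigger actor that starts and ends an interaction when actors begin and stop overlapping it.
; Overlap begin gets the interactor tag from the other actor through a message call and passes it to TryInteract, while overlap end calls TryEndInteraction.
; The Interact and EndInteraction events forward to the BPCInteractor component.
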(event Collision|EventActorBeginOverlap
  (params (OtherActor :type Actor%20Object%20Reference))
  (bind _interactor (Class|BPIInteractor|GetInteractorTag(Message) OtherActor))
  (CallFunction|TryInteract _interactor))

(event EventInteract
  (params (Interactor :type Gameplay%20Tag%20Structure))
  (Default|Interact (Variables|Default|GetBPC_Interactor) Interactor))

(event EventEndInteraction
  (Default|EndInteraction (Variables|Default|GetBPC_Interactor)))

(event Collision|EventActorEndOverlap
  (params (OtherActor :type Actor%20Object%20Reference))
  (CallFunction|TryEndInteraction))

(fn ConstructionScript
  (|CallParentFunction))